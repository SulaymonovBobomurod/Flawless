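; Base chest actor that stores items and animates its lid open or closed on interaction.
; An interact event picks open or close, playing or reversing a timeline that lerps the lid's rotation through MultiSetRelativeRotation.
; Add and remove events loop over the amount, storing each unit as its own ChestInventory array entry; adding also prints a debug string.
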(event Custom|CloseChest
  (bind _alphatrack (Timeline|OpenTimeline ReverseFromEnd)
    (:Update
      (CallFunction|MultiSetRelativeRotation (Math|Rotator|Lerp(Rotator) "0, 0, 0" "50.000000, 0, 0" _alphatrack)))))

(event Custom|MultiSetRelativeRotation
  (params (NewRotation :type Rotator))
  (Transformation|SetRelativeRotation (Variables|Default|GetLid) NewRotation false false))

(event Custom|OpenChest
  (bind _alphatrack (Timeline|OpenTimeline PlayFromStart)
    (:Update
      (CallFunction|MultiSetRelativeRotation (Math|Rotator|Lerp(Rotator) "0, 0, 0" "50.000000, 0, 0" _alphatrack)))))

(event EventBeginPlay)

(event Collision|EventActorBeginOverlap
  (params (OtherActor :type Actor%20Object%20Reference)))

(event EventTick
  (params (DeltaSeconds :type Float%20%28single-precision%29)))

(event EventCallChestInteract
  (params (Close :type Boolean))
  (if Close
    (CallFunction|CloseChest)
    (else
      (CallFunction|OpenChest))))

(event EventCallAddItemtoInteractable
  (params (Item%20To%20add :type BP%20Master%20Interactable%20Class%20Reference) (AmountToAdd :type Integer))
  (for _index (range 1 AmountToAdd)
    (Utilities|Array|Add (Variables|Default|GetChestInventory) Item%20To%20add)
    (Development|PrintString "Hello")))

(event EventCallRemoveChestItem
  (params (NewParam :type BP%20Master%20Interactable%20Class%20Reference) (Amount :type Integer))
  (bind _chestinventory (Variables|Default|GetChestInventory))
  (for _index (range 1 Amount)
    (Utilities|Array|RemoveIndex _chestinventory (Utilities|Array|FindItem _chestinventory NewParam))))

(fn ConstructionScript)